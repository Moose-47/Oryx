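; BP_PauseManager is an actor that opens the pause menu and pauses the game.
; It enables input from player 0 on BeginPlay, then listens for P or Escape.
; Either key creates a new WBP_PauseMenu, adds it to the viewport, pauses the game, switches to UI-only input and shows the mouse cursor.
; It contains no unpause logic.
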(event `self.ReceiveBeginPlay`
  (`self.EnableInput` (`GameplayStatics.GetPlayerController` 0)))

(event `Key|P`
  (params (Key :type "Key Structure"))
  (bind _returnvalue (`GameplayStatics.GetPlayerController` 0))
  (:`Pressed`
    (bind _returnvalue_2 (`|CreateWidget` "/Game/UI/WBP_PauseMenu.WBP_PauseMenu_C"))
    (`UserWidget.AddToViewport` _returnvalue_2 0)
    (`GameplayStatics.SetGamePaused` true)
    (`WidgetBlueprintLibrary.SetInputMode_UIOnlyEx` _returnvalue null :!label _label)
    (set `PlayerController.bShowMouseCursor` true _returnvalue)))

(event `Key|Escape`
  (params (Key :type "Key Structure"))
  (:`Pressed`
    (bind _returnvalue (`|CreateWidget` "/Game/UI/WBP_PauseMenu.WBP_PauseMenu_C"))
    (`UserWidget.AddToViewport` _returnvalue 0)
    (`GameplayStatics.SetGamePaused` true)
    (goto _label)))

(fn `UserConstructionScript`)